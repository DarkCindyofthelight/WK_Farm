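; BP_FarmTile_Auto1 is a farm tile Blueprint that plants a crop based on the player's selected seed.
; PlantSeed skips occupied tiles, reads Seed from the ThirdPersonCharacter, and handles only case 0, which calls PlantWheat and marks the tile planted.
; PlantWheat chains three static mesh component additions with destroys between them, leaving the last mesh in place, with no delays between the swaps.
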(event `PlantWheat`
  (bind _relativetransformlocation (`self.RelativeTransformLocation`))
  (`AddComponent|NODE_AddStaticMeshComponent-0` :`RelativeTransform` (`KismetMathLibrary.MakeTransform` _relativetransformlocation))
  (`ActorComponent.K2_DestroyComponent`)
  (`AddComponent|NODE_AddStaticMeshComponent-1` :`RelativeTransform` (`KismetMathLibrary.MakeTransform` _relativetransformlocation))
  (`ActorComponent.K2_DestroyComponent`)
  (`AddComponent|NODE_AddStaticMeshComponent-2` :`RelativeTransform` (`KismetMathLibrary.MakeTransform` _relativetransformlocation)))

(event `/Game/Geometry/Blueprint/BPI_PlantSee.PlantSeed`
  (if (not (`self.IsSomethingPlanted?`))
    (bind _asthird_person_character (cast `/Game/ThirdPersonBP/Blueprints/ThirdPersonCharacter` (`GameplayStatics.GetPlayerCharacter` 0)))
    (switch `int` (`/Game/ThirdPersonBP/Blueprints/ThirdPersonCharacter.Seed` _asthird_person_character)
      (:`0`
        (`self.PlantWheat`)
        (set `self.IsSomethingPlanted?` true)))))

(fn `UserConstructionScript`)